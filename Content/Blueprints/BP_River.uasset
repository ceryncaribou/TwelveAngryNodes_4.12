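; River actor that builds itself procedurally in the construction script from an array of world points.
; GenerateRiver turns the points into a spline and lays fixed-length spline meshes along it, randomly picking mesh variants and blocking Visibility traces.
; Slight random width jitter carries each segment's end scale into the next start, keeping joints seamless.
; BeginningID and EndingID choose which termination types get a static mesh aligned to the end points.
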(event EventBeginPlay)

(fn ConstructionScript
  (Spline|ClearSplinePoints (Variables|Default|GetRiverSpline))
  (CallFunction|GenerateRiver (Variables|Default|GetPointsArray)))

(fn GenerateRiver
  (params (PointsArray :type Array%20of%20Vectors))
  (bind _riverspline (Variables|Default|GetRiverSpline))
  (bind _tangentscale (Variables|Default|GetTangentScale))
  (bind _riverspline_2 (Variables|Default|GetRiverSpline))
  (bind _item (Utilities|Array|Get(acopy) (Variables|Default|GetPointsArray)))
  (bind _returnvalue (Utilities|Array|LastIndex (Variables|Default|GetPointsArray)))
  (bind _returnvalue_2 (Utilities|Array|LastIndex (Variables|Default|GetPointsArray)))
  (bind _returnvalue_3 (Utilities|Array|LastIndex (Variables|Default|GetPointsArray)))
  (bind _item_2 (Utilities|Array|Get(acopy) (Variables|Default|GetPointsArray)))
  (bind _item_3 (Utilities|Array|Get(acopy) (Variables|Default|GetPointsArray)))
  (bind _item_4 (Utilities|Array|Get(acopy) (Variables|Default|GetPointsArray) _returnvalue))
  (bind _item_5 (Utilities|Array|Get(acopy) (Variables|Default|GetPointsArray) _returnvalue_3))
  (bind _item_6 (Utilities|Array|Get(acopy) (Variables|Default|GetPointsArray) _returnvalue_2))
  (Class|SplineComponent|SetSplineWorldPoints _riverspline_2 PointsArray)
  (LocalVariables|SetTempXScale (Math|Random|RandomFloatinRange 0.95 1.05))
  (LocalVariables|SetLastIndex (.ReturnValue (Math|Float|Division(WholeandRemainder) (Spline|GetSplineLength _riverspline_2) (Variables|Default|GetMeshLength))))
  (for _index (range 0 (LocalVariables|GetLastIndex))
    (LocalVariables|SetTempIndex _index)
    (bind _returnvalue_4 (AddComponent|AddSplineMeshComponent true))
    (LocalVariables|SetCurrentSM _returnvalue_4)
    (SplineMesh|SetStartScale (LocalVariables|GetCurrentSM) (Math|Vector2D|MakeVector2D 1.0 (LocalVariables|GetTempXScale)) :!class /Script/Engine.SplineMeshComponent)
    (LocalVariables|SetTempXScale (Math|Random|RandomFloatinRange 0.95 1.05))
    (SplineMesh|SetEndScale (LocalVariables|GetCurrentSM) (Math|Vector2D|MakeVector2D 1.0 (LocalVariables|GetTempXScale)) :!class /Script/Engine.SplineMeshComponent)
    ;[1 1 1] River body
    (switch int (Math|Random|RandomIntegerinRange 0 9)
      (:Default
        _)
      (:0
        (Components|StaticMesh|SetStaticMesh (LocalVariables|GetCurrentSM) "/Game/StaticMeshes/SM_River4.SM_River4" :!label _label))
      (:1
        _)
      (:2
        _)
      (:3
        _)
      (:4
        _)
      (:5
        (Components|StaticMesh|SetStaticMesh (LocalVariables|GetCurrentSM) "/Game/StaticMeshes/SM_River2.SM_River2" :!label _label_2))
      (:6
        (goto _label_2))
      (:7
        (Components|StaticMesh|SetStaticMesh (LocalVariables|GetCurrentSM) "/Game/StaticMeshes/SM_River3.SM_River3" :!label _label_3))
      (:8
        (goto _label_3))
      (:9
        (goto _label)))
    (Collision|SetCollisionResponsetoChannel (LocalVariables|GetCurrentSM) "ECC_Visibility" "ECR_Block")
    (SplineMesh|SetStartandEnd _returnvalue_4 (Class|SplineComponent|GetWorldLocationatDistanceAlongSpline _riverspline (* _index (Variables|Default|GetMeshLength))) (* (Class|SplineComponent|GetWorldDirectionatDistanceAlongSpline _riverspline (* _index (Variables|Default|GetMeshLength))) _tangentscale) (Class|SplineComponent|GetWorldLocationatDistanceAlongSpline _riverspline (* (+ _index 1) (Variables|Default|GetMeshLength))) (* (Class|SplineComponent|GetWorldDirectionatDistanceAlongSpline _riverspline (* (+ _index 1) (Variables|Default|GetMeshLength))) _tangentscale) :!class /Script/Engine.SplineMeshComponent))
  (Utilities|FlowControl|Sequence
    (:then_0
      (switch int (Variables|Default|GetBeginningID)
        (:0
          (AddComponent|AddStaticMeshComponent true (Math|Transform|MakeTransform _item (Math|Rotator|CombineRotators (Math|Rotator|FindLookatRotation _item (Utilities|Array|Get(acopy) (Variables|Default|GetPointsArray) 1)) "0,90.000000, 0") "1,1.000000,1")))
        (:2
          (AddComponent|AddStaticMeshComponent false (Math|Transform|MakeTransform _item_2 (Math|Rotator|CombineRotators (Math|Rotator|FindLookatRotation _item_2 (Utilities|Array|Get(acopy) (Variables|Default|GetPointsArray) 1)) "0,90.000000, 0") "1,1.000000,1")))
        (:3
          (AddComponent|AddStaticMeshComponent false (Math|Transform|MakeTransform _item_3 (Math|Rotator|CombineRotators (Math|Rotator|FindLookatRotation _item_3 (Utilities|Array|Get(acopy) (Variables|Default|GetPointsArray) 1)) "0,90.000000, 0") "1,1.000000,1")))))
    (:then_1
      (switch int (Variables|Default|GetEndingID) ; 0 = river source // 1 = fork // 2 = cascade & chute // 3 = lake
        (:0
          (AddComponent|AddStaticMeshComponent true (Math|Transform|MakeTransform _item_4 (Math|Rotator|CombineRotators (Math|Rotator|FindLookatRotation (Utilities|Array|Get(acopy) (Variables|Default|GetPointsArray) (- _returnvalue 1)) _item_4) "0,-90.000000, 0") "1,1.000000,1")))
        (:2
          (AddComponent|AddStaticMeshComponent true (Math|Transform|MakeTransform _item_5 (Math|Rotator|CombineRotators (Math|Rotator|FindLookatRotation (Utilities|Array|Get(acopy) (Variables|Default|GetPointsArray) (- _returnvalue_3 1)) _item_5) "0,-90.000000, 0") "1,1.000000,1") :!label _label_4))
        (:3
          (goto _label_4))
        (:4
          (AddComponent|AddStaticMeshComponent true (Math|Transform|MakeTransform _item_6 (Math|Rotator|CombineRotators (Math|Rotator|FindLookatRotation (Utilities|Array|Get(acopy) (Variables|Default|GetPointsArray) (- _returnvalue_2 1)) _item_6) "0,-90.000000, 0") "1,1.000000,1")))))))