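; GameOverseer is the bootstrap actor that sets up a game session on BeginPlay.
; It spawns the GameManager with a hardcoded player setup, then a GameCamera and MapGenerator that share a fixed map size, with the generator also receiving the manager.
; It hands the camera to the manager, makes it the view target and passes camera, manager and itself to MyPlayerController.
; CleanUp destroys only the MapGenerator.
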(event EventBeginPlay
  (bind _returnvalue (Math|Transform|MakeTransform "0, 0, 0"))
  (bind _returnvalue_2 (Game|GetPlayerController 0))
  (bind _returnvalue_3 (Game|SpawnActorfromClass "/Game/Blueprints/GameManager.GameManager_C" _returnvalue true 0 self 2 0))
  (Variables|Default|SetGameManager _returnvalue_3)
  (Variables|Default|SetMapsizex 35)
  (Variables|Default|SetMapsizey 25)
  (bind _returnvalue_4 (Game|SpawnActorfromClass "/Game/Blueprints/GameCamera.GameCamera_C" _returnvalue true 0 (Variables|Default|GetMapsizex) (Variables|Default|GetMapsizey)))
  (Variables|Default|SetGame%20Camera _returnvalue_4)
  (bind _returnvalue_5 (Game|SpawnActorfromClass "/Game/Blueprints/MapGenerator.MapGenerator_C" _returnvalue true 0 self (Variables|Default|GetMapsizex) (Variables|Default|GetMapsizey) (Variables|Default|GetGameManager)))
  (Variables|Default|SetMapGenerator _returnvalue_5)
  (Default|InitializeGameCamera (Variables|Default|GetGameManager) (Variables|Default|GetGame%20Camera))
  (Game|Player|SetViewTargetwithBlend _returnvalue_2 (Variables|Default|GetGame%20Camera) 0.0 "VTBlend_Linear" 0.0 false)
  (bind _asmy_player_controller (Utilities|Casting|CastToMyPlayerController _returnvalue_2))
  (Default|SetGameCamera _asmy_player_controller (Variables|Default|GetGame%20Camera))
  (Default|SetGameManager _asmy_player_controller (Variables|Default|GetGameManager))
  (Default|SetGameOverseer _asmy_player_controller self))

(fn ConstructionScript)

(fn CleanUp
  (Actor|DestroyActor (Variables|Default|GetMapGenerator)))