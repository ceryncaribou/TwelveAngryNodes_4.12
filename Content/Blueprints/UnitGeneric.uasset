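; Generic unit Blueprint with selection-driven visibility and mirrored copies, apparently for a horizontally wrapping hex map.
; The construction script offsets positive and negative meshes by plus and minus the map width along Y (Mapsizex times 100√3), with select circles raised slightly in Z.
; Tick toggles three components, likely the selection circles, to match IsSelected, using IsVisible to act only on changes.
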(event EventTick
  (params (DeltaSeconds :type Float%20%28single-precision%29))
  (if (Variables|Default|GetisSelected)
    (if (not (Variables|Default|GetisVisible))
      (Rendering|SetVisibility true false)
      (Rendering|SetVisibility true false)
      (Rendering|SetVisibility true false)
      (Variables|Default|SetisVisible true))
    (elif (Variables|Default|GetisVisible)
      (Rendering|SetVisibility false false)
      (Rendering|SetVisibility false false)
      (Rendering|SetVisibility false false)
      (Variables|Default|SetisVisible false))))

(fn ConstructionScript
  (bind _mapsizex (Variables|Default|Getmapsizex))
  (bind _returnvalue (* _mapsizex 173.205080756888))
  (bind _returnvalue_2 (Math|Vector|MakeVector 0.0 _returnvalue 0.0))
  (bind _returnvalue_3 (* _returnvalue_2 -1.0))
  (Transformation|SetRelativeLocation (Variables|Default|GetPositiveMesh) _returnvalue_2 false)
  (Transformation|SetRelativeLocation (Variables|Default|GetPosSelectCircle) (+ _returnvalue_2 "0, 0,10.000000") false)
  (Transformation|SetRelativeLocation (Variables|Default|GetNegativeMesh) _returnvalue_3 false)
  (Transformation|SetRelativeLocation (Variables|Default|GetNegSelectCircle) (+ _returnvalue_3 "0, 0,10.000000") false))