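; Player controller for a turn-based civilization game, turning mouse and input actions into camera control and commands for the current player.
; Tick edge-scrolls GameCamera near viewport borders, with flags letting held movement inputs override it, while zoom inputs drive the camera directly.
; Clicks go to the current CivManagerPlayer from GameManager, using a delayed counter to detect double-click selection and printing when an AI is active.
; End-turn input triggers the current civ manager.
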(event EventTick
  (params (DeltaSeconds :type Float%20%28single-precision%29))
  (bind (_locationx _locationy) (Game|Player|GetMousePosition))
  (bind _returnvalue (Viewport|GetViewportSize))
  (bind _gamecamera (Variables|Default|GetGameCamera))
  (bind (_x _y) (Math|Vector2D|BreakVector2D _returnvalue))
  (bind _returnvalue_2 (/ _locationy _y))
  (bind _returnvalue_3 (/ _locationx _x))
  ;[1 1 1] Sidescrolling
  (if (Variables|Default|GetMovingDown)
    _
    (else
      (Default|MoveDown _gamecamera (> _returnvalue_2 0.97))))
  (if (Variables|Default|GetMovingUp)
    _
    (else
      (Default|MoveUp _gamecamera (< _returnvalue_2 0.03))))
  (if (Variables|Default|GetMovingLeft)
    _
    (else
      (Default|MoveLeft _gamecamera (< _returnvalue_3 0.03))))
  (if (not (Variables|Default|GetMovingRight))
    (Default|MoveRight _gamecamera (> _returnvalue_3 0.97))))

(event EventBeginPlay
  (Variables|Default|SetMovingDown false)
  (Variables|Default|SetMovingUp false)
  (Variables|Default|SetMovingLeft false)
  (Variables|Default|SetMovingRight false))

(event Input|ActionEvents|InputActionMoveUp
  (bind _gamecamera (Variables|Default|GetGameCamera))
  ;[1 1 1] Camera Movement
  (:Pressed
    (Default|MoveUp _gamecamera true)
    (Variables|Default|SetMovingUp true))
  (:Released
    (Default|MoveUp _gamecamera false)
    (Variables|Default|SetMovingUp false)))

(event Input|ActionEvents|InputActionEndTurn
  (bind _gamemanager (Variables|Default|GetGameManager))
  ;[1 1 1] Turn end
  (:Pressed
    (Class|CCivManagerInterface|EndTurnTriggered (Utilities|Array|Get(acopy) (Variables|/Game/Blueprints/GameManager.GameManager_C|GetCivManagerList _gamemanager) (Variables|/Script/TwelveAngryNodes.C_GameManager|GetcurrentPlayer _gamemanager)))))

(event Input|ActionEvents|InputActionZoomIn
  (bind _gamecamera (Variables|Default|GetGameCamera))
  ;[1 1 1] Camera Movement
  (:Pressed
    (Default|Zoomin _gamecamera true)
    (Default|Zoom _gamecamera))
  (:Released
    (Default|Zoomin _gamecamera false)))

(event Input|ActionEvents|InputActionZoomOut
  (bind _gamecamera (Variables|Default|GetGameCamera))
  ;[1 1 1] Camera Movement
  (:Pressed
    (Default|ZoomOut _gamecamera true)
    (Default|DeZoom _gamecamera))
  (:Released
    (Default|ZoomOut _gamecamera false)))

(event Input|ActionEvents|InputActionMoveDown
  (bind _gamecamera (Variables|Default|GetGameCamera))
  ;[1 1 1] Camera Movement
  (:Pressed
    (Default|MoveDown _gamecamera true)
    (Variables|Default|SetMovingDown true))
  (:Released
    (Default|MoveDown _gamecamera false)
    (Variables|Default|SetMovingDown false)))

(event Input|ActionEvents|InputActionMoveRight
  (bind _gamecamera (Variables|Default|GetGameCamera))
  ;[1 1 1] Camera Movement
  (:Pressed
    (Default|MoveRight _gamecamera true)
    (Variables|Default|SetMovingRight true))
  (:Released
    (Default|MoveRight _gamecamera false)
    (Variables|Default|SetMovingRight false)))

(event Input|ActionEvents|InputActionClickSelect
  (bind _gamemanager (Variables|Default|GetGameManager))
  ;[1 1 1] Mouse clicks
  (:Pressed
    (Variables|Default|SetLeftClickCount (+ (Variables|Default|GetLeftClickCount) 1))
    (Utilities|FlowControl|Delay 0.25)
    (if (> (Variables|Default|GetLeftClickCount) 1)
      (Variables|Default|SetdoubleClick true)
      (Development|PrintString "double click BIATCH")
      (else
        (Variables|Default|SetdoubleClick false)))
    (Variables|Default|SetLeftClickCount 0)
    (bind _asciv_manager_player (Utilities|Casting|CastToCivManagerPlayer (Utilities|Array|Get(acopy) (Variables|/Game/Blueprints/GameManager.GameManager_C|GetCivManagerList _gamemanager) (Variables|/Script/TwelveAngryNodes.C_GameManager|GetcurrentPlayer _gamemanager)))
      (:then
        (Default|NewSelection _asciv_manager_player (Variables|Default|GetdoubleClick)))
      (:CastFailed
        (Development|PrintString "current player is AI")))))

(event Input|ActionEvents|InputActionClickAct
  (bind _gamemanager (Variables|Default|GetGameManager))
  (bind _civmanagerlist (Variables|/Game/Blueprints/GameManager.GameManager_C|GetCivManagerList _gamemanager))
  (bind _currentplayer (Variables|/Script/TwelveAngryNodes.C_GameManager|GetcurrentPlayer _gamemanager))
  (bind _item (Utilities|Array|Get(acopy) _civmanagerlist _currentplayer))
  ;[1 1 1] Mouse clicks
  (:Pressed
    (bind _asciv_manager_player (Utilities|Casting|CastToCivManagerPlayer _item)
      (:then
        (Variables|/Game/Blueprints/CivManagerPlayer.CivManagerPlayer_C|SetRightClicking _asciv_manager_player true))
      (:CastFailed
        (Development|PrintString "current player is AI" :!label _label))))
  (:Released
    (bind _asciv_manager_player_2 (Utilities|Casting|CastToCivManagerPlayer _item)
      (:then
        (Variables|/Game/Blueprints/CivManagerPlayer.CivManagerPlayer_C|SetRightClicking _asciv_manager_player_2 false))
      (:CastFailed
        (goto _label)))))

(event Input|ActionEvents|InputActionMoveLeft
  (bind _gamecamera (Variables|Default|GetGameCamera))
  ;[1 1 1] Camera Movement
  (:Pressed
    (Default|MoveLeft _gamecamera true)
    (Variables|Default|SetMovingLeft true))
  (:Released
    (Default|MoveLeft _gamecamera false)
    (Variables|Default|SetMovingLeft false)))

(fn ConstructionScript)

(fn SetGameCamera
  (params (Camera :type Game%20Camera%20Object%20Reference))
  (Variables|Default|SetGameCamera Camera))

(fn SetGameOverseer
  (params (Overseer :type Game%20Overseer%20Object%20Reference))
  (Variables|Default|SetGameOverseer Overseer))

(fn SetGameManager
  (params (Manager :type Game%20Manager%20Object%20Reference))
  (Variables|Default|SetGameManager Manager))