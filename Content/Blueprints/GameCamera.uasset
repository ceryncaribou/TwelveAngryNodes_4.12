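; Map camera that pans and zooms over the play area, wrapping around horizontally at the left and right edges.
; BeginPlay derives limits from map size and spawns fluorescent marker lines.
; Setter functions toggle movement flags that Tick applies, clamping vertical panning and scaling pan speed with height.
; Zooming changes height within limits and recomputes pitch from it; Zoom and DeZoom events trigger single steps of the same logic.
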(event Custom|Zoom
  ;[1 1 1] Checking limits of map
  (if (> (.Z (Math|Vector|BreakVector (Variables|Default|GetPositionVector))) (Variables|Default|GetZmin))
    ;[1 1 1] Moving Camera
    (Variables|Default|SetPositionVector (+ (Variables|Default|GetPositionVector) (* "0.000000,0.000000,-1.000000" (* (Variables|Default|GetZoomSpeed) (Variables|Default|GetDeltaSeconds)))))
    (Transformation|SetWorldRotation (Math|Vector|RotatorfromAxisandAngle "0,1.000000, 0" (Class|KismetMathLibrary|DegAtan2 (.Z (Math|Vector|BreakVector (Variables|Default|GetPositionVector))) 461.8802153517005)) false)))

(event Custom|DeZoom
  ;[1 1 1] Checking limits of map
  (if (< (.Z (Math|Vector|BreakVector (Variables|Default|GetPositionVector))) (Variables|Default|GetZmax))
    ;[1 1 1] Moving Camera
    (Variables|Default|SetPositionVector (+ (Variables|Default|GetPositionVector) (* "0.000000,0.000000,1.000000" (* (Variables|Default|GetZoomSpeed) (Variables|Default|GetDeltaSeconds)))))
    (Transformation|SetWorldRotation (Math|Vector|RotatorfromAxisandAngle "0,1.000000, 0" (Class|KismetMathLibrary|DegAtan2 (.Z (Math|Vector|BreakVector (Variables|Default|GetPositionVector))) 461.8802153517005)) false)))

(event EventTick
  (params (DeltaSeconds :type Float%20%28single-precision%29))
  (Variables|Default|SetDeltaSeconds DeltaSeconds)
  (Utilities|FlowControl|Sequence
    (:then_0
      (if (Variables|Default|GetIsMovingUp)
        ;[1 1 1] Checking limits of map
        (if (< (.X (Math|Vector|BreakVector (Variables|Default|GetPositionVector))) (Variables|Default|GetTopLimit))
          ;[1 1 1] Moving Camera
          (Variables|Default|SetPositionVector (+ (Variables|Default|GetPositionVector) (* "1.000000, 0, 0" (* (* (Variables|Default|GetCameraSpeed) (Variables|Default|GetDeltaSeconds)) (/ (.Z (Math|Vector|BreakVector (Variables|Default|GetPositionVector))) 8e+02))))))))
    (:then_1
      (if (Variables|Default|GetIsMovingDown)
        (if (> (.X (Math|Vector|BreakVector (Variables|Default|GetPositionVector))) (Variables|Default|GetBotLimit))
          (Variables|Default|SetPositionVector (+ (Variables|Default|GetPositionVector) (* "-1.000000, 0, 0" (* (* (Variables|Default|GetCameraSpeed) (Variables|Default|GetDeltaSeconds)) (/ (.Z (Math|Vector|BreakVector (Variables|Default|GetPositionVector))) 8e+02))))))))
    (:then_2
      (if (Variables|Default|GetIsMovingRight)
        (if (< (.Y (Math|Vector|BreakVector (Variables|Default|GetPositionVector))) (Variables|Default|GetRightLimit))
          (Variables|Default|SetPositionVector (+ (Variables|Default|GetPositionVector) (* "0.000000,1.000000, 0" (* (* (Variables|Default|GetCameraSpeed) (Variables|Default|GetDeltaSeconds)) (/ (.Z (Math|Vector|BreakVector (Variables|Default|GetPositionVector))) 8e+02)))))
          (else
            (Variables|Default|SetPositionVector (+ (Variables|Default|GetPositionVector) (* "0.000000,-1.000000, 0" (Variables|Default|GetRightLimit))))))))
    (:then_3
      (if (Variables|Default|GetIsMovingLeft)
        (if (> (.Y (Math|Vector|BreakVector (Variables|Default|GetPositionVector))) (Variables|Default|GetLeftLimit))
          (Variables|Default|SetPositionVector (+ (Variables|Default|GetPositionVector) (* "0.000000,-1.000000,0.000000" (* (* (Variables|Default|GetCameraSpeed) (Variables|Default|GetDeltaSeconds)) (/ (.Z (Math|Vector|BreakVector (Variables|Default|GetPositionVector))) 8e+02)))))
          (else
            (Variables|Default|SetPositionVector (+ (Variables|Default|GetPositionVector) (* "0.000000,1.000000, 0" (Variables|Default|GetRightLimit))))))))
    (:then_4
      (if (Variables|Default|GetIsZoomingIn)
        (if (> (.Z (Math|Vector|BreakVector (Variables|Default|GetPositionVector))) (Variables|Default|GetZmin))
          (Variables|Default|SetPositionVector (+ (Variables|Default|GetPositionVector) (* "0.000000,0.000000,-1.000000" (* (Variables|Default|GetZoomSpeed) (Variables|Default|GetDeltaSeconds)))))
          (Transformation|SetWorldRotation (Math|Vector|RotatorfromAxisandAngle "0,1.000000, 0" (Class|KismetMathLibrary|DegAtan2 (.Z (Math|Vector|BreakVector (Variables|Default|GetPositionVector))) 461.8802153517005)) false :!label _label))))
    (:then_5
      (if (Variables|Default|GetIsZoomingOut)
        (if (< (.Z (Math|Vector|BreakVector (Variables|Default|GetPositionVector))) (Variables|Default|GetZmax))
          (Variables|Default|SetPositionVector (+ (Variables|Default|GetPositionVector) (* "0.000000,0.000000,1.000000" (* (Variables|Default|GetZoomSpeed) (Variables|Default|GetDeltaSeconds)))))
          (goto _label))))
    (:then_6
      (Transformation|SetActorLocation (Variables|Default|GetPositionVector) false))))

(event EventBeginPlay
  (Variables|Default|SetTopLimit (* (- (Variables|Default|GetMapsizey) 8) 1.5e+02))
  (Variables|Default|SetRightLimit (* (Variables|Default|GetMapsizex) 173.205080756888))
  (Game|SpawnActorfromClass "/Game/Blueprints/LongAssFluoLine.LongAssFluoLine_C" (Math|Transform|MakeTransform "0.000000, 0,75.000000" "0, 0, 0" "1000.000000,0.010000,1") false 0 true 0)
  (Game|SpawnActorfromClass "/Game/Blueprints/LongAssFluoLine.LongAssFluoLine_C" (Math|Transform|MakeTransform (Math|Vector|MakeVector 0.0 (Variables|Default|GetRightLimit) 75.0) "0, 0, 0" "1000.000000,0.010000,1") false 0 true 0)
  (Game|SpawnActorfromClass "/Game/Blueprints/LongAssFluoLine.LongAssFluoLine_C" (Math|Transform|MakeTransform (Math|Vector|MakeVector 0.0 (* (- (Variables|Default|GetMapsizey) 1) 86.602540378444) 75.0) "0, 0, 0" "1000.000000,0.010000,1") false 0 false 0))

(fn ConstructionScript)

(fn MoveUp
  (params (Enable :type Boolean))
  (Variables|Default|SetIsMovingUp Enable))

(fn MoveDown
  (params (Enable :type Boolean))
  (Variables|Default|SetIsMovingDown Enable))

(fn MoveRight
  (params (Enable :type Boolean))
  (Variables|Default|SetIsMovingRight Enable))

(fn MoveLeft
  (params (Enable :type Boolean))
  (Variables|Default|SetIsMovingLeft Enable))

(fn Zoomin
  (params (Enable :type Boolean))
  (Variables|Default|SetIsZoomingIn Enable))

(fn ZoomOut
  (params (Enable :type Boolean))
  (Variables|Default|SetIsZoomingOut Enable))