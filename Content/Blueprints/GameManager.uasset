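; Game manager for a turn-based, hex-map civilization game that sets up human and AI CivManagers with starting units.
; Tick polls the current CivManager's done flag to advance players, refilling unit moves after each full round.
; It also handles unit spawning and movement, city founding and improvements.
; Hex changes are mirrored onto positive and negative twin tiles, with visuals refreshed from the current player's map arrays.
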(event EventTick
  (params (DeltaSeconds :type Float%20%28single-precision%29))
  (CallFunction|CheckifEndOfTurn))

(fn ConstructionScript)

(fn InitializeGameCamera
  (params (Camera :type Game%20Camera%20Object%20Reference))
  (Variables|Default|SetCamera Camera))

(fn InitializeCivManagers
  (params (HumanPlayers :type Integer) (AIPlayers :type Integer))
  (bind _returnvalue (Math|Transform|MakeTransform "0, 0, 0"))
  (bind _civmanagerlist (Variables|Default|GetCivManagerList))
  (for _index (range 1 HumanPlayers)
    (bind _returnvalue_2 (Game|SpawnActorfromClass "/Game/Blueprints/CivManagerPlayer.CivManagerPlayer_C" _returnvalue true 0 self (- _index 1)))
    (Utilities|Array|Add _civmanagerlist _returnvalue_2))
  (for _index_2 (range 1 AIPlayers)
    (bind _returnvalue_3 (Game|SpawnActorfromClass "/Game/Blueprints/CivManagerAI.CivManagerAI_C" _returnvalue false 0 self (+ _index_2 HumanPlayers -1)))
    (Utilities|Array|Add _civmanagerlist _returnvalue_3))
  (for (_array_element _array_index) (Variables|Default|GetCivManagerList)
    (Class|CCivManagerInterface|InitializeCivManagerMapArrays _array_element)
    (CallFunction|SpawnStartingUnits _array_index)))

(fn InitializeGame
  (CallFunction|InitializeCivManagers (Variables|Default|GetNumberOfPlayers) (Variables|Default|GetNumberOfAIs))
  (CallFunction|PositionCameraonHex (Utilities|Array|Get(acopy) (Variables|Default|GetStartingSpots)))
  (Variables|Default|SetcurrentTurn 1)
  (Variables|Default|SetcurrentPlayer 0)
  ;[1 1 1] Game Begins!
  (Class|CCivManagerInterface|BeginTurn (Utilities|Array|Get(acopy) (Variables|Default|GetCivManagerList) (Variables|Default|GetcurrentPlayer))))

(fn PositionCameraonHex
  (params (New%20Position :type Integer))
  (bind _mapsizex (Variables|Default|Getmapsizex))
  (bind _returnvalue (/ New%20Position _mapsizex))
  (Variables|/Game/Blueprints/GameCamera.GameCamera_C|SetPositionVector (Variables|Default|GetCamera) (Math|Vector|MakeVector (- (* _returnvalue 1.5e+02) 461.8802153517005) (+ (* (Math|Integer|%(Integer) New%20Position _mapsizex) 173.205080756888) (* _returnvalue 86.602540378444)) 8e+02)))

(fn MoveUnitfromAtoB
  (params (Hex%20A :type Integer) (Hex%20B :type Integer) (Unit :type C%20Unit%20Generic%20Object%20Reference))
  (bind _primaryhexarray (Variables|Default|GetPrimaryHexArray))
  (bind _hasnegativetwin (Variables|Default|GethasNegativeTwin))
  (bind _haspositivetwin (Variables|Default|GethasPositiveTwin))
  (Transformation|SetActorLocation Unit (Transformation|GetActorLocation (Utilities|Array|Get(acopy) (Variables|Default|GetPrimaryHexArray) Hex%20B)) false)
  (Development|PrintString "ici?")
  ;[1 1 1] Updating unit list information in both hexes, plus positive and negative twins
  (Utilities|Array|RemoveItem (Variables|/Script/TwelveAngryNodes.C_HexTile|GetUnitListOnHex (Utilities|Array|Get(acopy) _primaryhexarray Hex%20A)) Unit)
  (Utilities|Array|Add (Variables|/Script/TwelveAngryNodes.C_HexTile|GetUnitListOnHex (Utilities|Array|Get(acopy) _primaryhexarray Hex%20B)) Unit)
  (if (Utilities|Array|Get(acopy) _hasnegativetwin Hex%20A)
    (Utilities|Array|RemoveItem (Variables|/Script/TwelveAngryNodes.C_HexTile|GetUnitListOnHex (Utilities|Array|Get(acopy) (Variables|Default|GetNegativeTwinHexArray) Hex%20A)) Unit))
  (if (Utilities|Array|Get(acopy) _hasnegativetwin Hex%20B)
    (Utilities|Array|Add (Variables|/Script/TwelveAngryNodes.C_HexTile|GetUnitListOnHex (Utilities|Array|Get(acopy) (Variables|Default|GetNegativeTwinHexArray) Hex%20B)) Unit))
  (if (Utilities|Array|Get(acopy) _haspositivetwin Hex%20A)
    (Utilities|Array|RemoveItem (Variables|/Script/TwelveAngryNodes.C_HexTile|GetUnitListOnHex (Utilities|Array|Get(acopy) (Variables|Default|GetPositiveTwinHexArray) Hex%20A)) Unit))
  (if (Utilities|Array|Get(acopy) _haspositivetwin Hex%20B)
    (Utilities|Array|Add (Variables|/Script/TwelveAngryNodes.C_HexTile|GetUnitListOnHex (Utilities|Array|Get(acopy) (Variables|Default|GetPositiveTwinHexArray) Hex%20B)) Unit)))

(fn EndOfTurn
  (Variables|Default|SetcurrentTurn (+ (Variables|Default|GetcurrentTurn) 1))
  (Variables|Default|SetcurrentPlayer 0)
  (for _array_element (Variables|Default|GetCivManagerList)
    (Variables|/Script/TwelveAngryNodes.C_CivManagerInterface|SetturnIsDone _array_element false)
    (for _array_element_2 (Variables|/Script/TwelveAngryNodes.C_CivManagerInterface|GetCivUnitList _array_element)
      (Variables|/Script/TwelveAngryNodes.C_UnitGeneric|SetremainingMoves _array_element_2 (Variables|/Script/TwelveAngryNodes.C_UnitGeneric|GetmaxMoves _array_element_2))))
  (Development|PrintString "starting next turn")
  (Development|PrintString (Utilities|String|ToString(Integer) (Variables|Default|GetcurrentTurn))))

(fn SpawnStartingUnits
  (params (Civ%20ID :type Integer))
  (bind _startingspots (Variables|Default|GetStartingSpots))
  (bind _item (Utilities|Array|Get(acopy) _startingspots Civ%20ID))
  (CallFunction|SpawnUnit Civ%20ID _item)
  (CallFunction|SpawnUnit Civ%20ID (+ _item 1)))

(fn SpawnUnit
  (params (OwnerIndex :type Integer) (Position :type Integer))
  (bind _primaryhexarray (Variables|Default|GetPrimaryHexArray))
  (bind _civmanagerlist (Variables|Default|GetCivManagerList))
  (bind _item (Utilities|Array|Get(acopy) _civmanagerlist OwnerIndex))
  (bind _item_2 (Utilities|Array|Get(acopy) _primaryhexarray Position))
  (bind _civunitlist (Variables|/Script/TwelveAngryNodes.C_CivManagerInterface|GetCivUnitList _item))
  (bind _returnvalue (Game|SpawnActorfromClass "/Game/Blueprints/UnitGeneric.UnitGeneric_C" (Math|Transform|MakeTransform (Transformation|GetActorLocation _item_2)) true 0 (Variables|Default|Getmapsizex) Position OwnerIndex (Utilities|Array|Length _civunitlist)))
  (Variables|/Script/TwelveAngryNodes.C_UnitGeneric|SetmaxMoves _returnvalue 2.0)
  (Variables|/Script/TwelveAngryNodes.C_UnitGeneric|SetremainingMoves _returnvalue 2.0)
  (Utilities|Array|Add _civunitlist _returnvalue)
  (Utilities|Array|Add (Variables|/Script/TwelveAngryNodes.C_HexTile|GetUnitListOnHex _item_2) _returnvalue)
  (if (Utilities|Array|Get(acopy) (Variables|Default|GethasPositiveTwin) Position)
    (Utilities|Array|Add (Variables|/Script/TwelveAngryNodes.C_HexTile|GetUnitListOnHex (Utilities|Array|Get(acopy) (Variables|Default|GetPositiveTwinHexArray) Position)) _returnvalue))
  (if (Utilities|Array|Get(acopy) (Variables|Default|GethasNegativeTwin) Position)
    (Utilities|Array|Add (Variables|/Script/TwelveAngryNodes.C_HexTile|GetUnitListOnHex (Utilities|Array|Get(acopy) (Variables|Default|GetNegativeTwinHexArray) Position)) _returnvalue)))

(fn CheckifEndOfTurn
  (if (Variables|/Script/TwelveAngryNodes.C_CivManagerInterface|GetturnIsDone (Utilities|Array|Get(acopy) (Variables|Default|GetCivManagerList) (Variables|Default|GetcurrentPlayer)))
    (Variables|Default|SetcurrentPlayer (+ (Variables|Default|GetcurrentPlayer) 1))
    (if (< (Variables|Default|GetcurrentPlayer) (+ (Variables|Default|GetNumberOfPlayers) (Variables|Default|GetNumberOfAIs)))
      _
      (else
        (CallFunction|EndOfTurn)))
    (Class|CCivManagerInterface|BeginTurn (Utilities|Array|Get(acopy) (Variables|Default|GetCivManagerList) (Variables|Default|GetcurrentPlayer)))
    (Development|PrintString (Utilities|String|Append "now playing : " (Utilities|String|ToString(Integer) (Variables|Default|GetcurrentPlayer))))))

(fn FoundCity
  (params (Owning%20Civ :type Integer) (Spawning%20Unit :type C%20Unit%20Generic%20Object%20Reference))
  (bind _civmanagerlist (Variables|Default|GetCivManagerList))
  (bind _position (Variables|/Script/TwelveAngryNodes.C_UnitGeneric|Getposition Spawning%20Unit))
  (bind _item (Utilities|Array|Get(acopy) _civmanagerlist Owning%20Civ))
  (bind _civcitylist (Variables|/Script/TwelveAngryNodes.C_CivManagerInterface|GetCivCityList _item))
  (bind _returnvalue (Game|SpawnActorfromClass "/Game/Blueprints/City.City_C" (Math|Transform|MakeTransform (Transformation|GetActorLocation Spawning%20Unit)) true 0 (Variables|Default|Getmapsizex) _position Owning%20Civ (Utilities|Array|Length _civcitylist) self))
  (bind _returnvalue_2 (Utilities|Array|Add _civcitylist _returnvalue))
  (Class|CCivManagerInterface|PlaceNewCity _item _position _returnvalue_2)
  (CallFunction|UpdateTile _position false true))

(fn UpdateTile
  (params (Tile%20Index :type Integer) (NeighboringTerrainChange :type Boolean) (Destroy%20Improvement :type Boolean))
  (bind _civmanagerlist (Variables|Default|GetCivManagerList))
  (bind _currentplayer (Variables|Default|GetcurrentPlayer))
  (bind _item (Utilities|Array|Get(acopy) _civmanagerlist _currentplayer))
  (bind _improvements (Variables|/Script/TwelveAngryNodes.C_CivManagerInterface|GetImprovements _item))
  (bind _revealedresources (Variables|/Script/TwelveAngryNodes.C_CivManagerInterface|GetrevealedResources _item))
  (bind _terraintype (Variables|/Script/TwelveAngryNodes.C_CivManagerInterface|GetTerrainType _item))
  (bind _altitudemap (Variables|/Script/TwelveAngryNodes.C_CivManagerInterface|GetAltitudeMap _item))
  (bind _item_2 (Utilities|Array|Get(acopy) _altitudemap Tile%20Index))
  (bind _item_3 (Utilities|Array|Get(acopy) _revealedresources Tile%20Index))
  (bind _item_4 (Utilities|Array|Get(acopy) _terraintype Tile%20Index))
  (bind _item_5 (Utilities|Array|Get(acopy) _improvements Tile%20Index))
  ;[1 1 1] PrimaryHex
  (bind _ashex_tile (Utilities|Casting|CastToHexTile (Utilities|Array|Get(acopy) (Variables|Default|GetPrimaryHexArray) Tile%20Index))
    (:then
      (Default|UpdateTileFeatures _ashex_tile _item_2 _item_4 _item_3 _item_5 NeighboringTerrainChange Destroy%20Improvement)
      ;[1 1 1] PositiveTwin
      (if (Utilities|Array|Get(acopy) (Variables|Default|GethasPositiveTwin) Tile%20Index)
        (bind _ashex_tile_2 (Utilities|Casting|CastToHexTile (Utilities|Array|Get(acopy) (Variables|Default|GetPositiveTwinHexArray) Tile%20Index))
          (:then
            (Default|UpdateTileFeatures _ashex_tile_2 _item_2 _item_4 _item_3 _item_5 NeighboringTerrainChange Destroy%20Improvement)
            ;[1 1 1] NegativeTwin
            (if (Utilities|Array|Get(acopy) (Variables|Default|GethasNegativeTwin) Tile%20Index) :!label _label
              (bind _ashex_tile_3 (Utilities|Casting|CastToHexTile (Utilities|Array|Get(acopy) (Variables|Default|GetNegativeTwinHexArray) Tile%20Index))
                (:then
                  (Default|UpdateTileFeatures _ashex_tile_3 _item_2 _item_4 _item_3 _item_5 NeighboringTerrainChange Destroy%20Improvement))
                (:CastFailed
                  (Development|PrintString "failed to  update negative twin")))))
          (:CastFailed
            (Development|PrintString "failed to update positive twin")))
        (else
          (goto _label))))
    (:CastFailed
      (Development|PrintString "failed cast to update primary hex"))))

(fn PlaceImprovement
  (params (Improvement :type EImprovement%20Enum :default "VE_None") (Tile%20Index :type Integer))
  (Class|CCivManagerInterface|PlaceNewImprovement (Utilities|Array|Get(acopy) (Variables|Default|GetCivManagerList) (Variables|Default|GetcurrentPlayer)) Tile%20Index Improvement)
  (CallFunction|UpdateTile Tile%20Index false (Utilities|Enum|Equal(Enum) Improvement "VE_None")))