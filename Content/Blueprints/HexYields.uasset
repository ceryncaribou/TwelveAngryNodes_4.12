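; HexYields displays a hex tile's food, production and gold yields as icons on a static mesh.
; Construction creates a dynamic instance of M_Yields, assigns it to the mesh, then calls UpdateYields with the three yield values.
; UpdateYields writes the amounts to material scalar parameters and sets icon X/Y offsets by which yields are nonzero, spreading two or three icons apart and centering otherwise.
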(fn ConstructionScript
  (bind _returnvalue (Rendering|Material|CreateDynamicMaterialInstance "/Game/Materials/Ui/M_Yields.M_Yields" :!class /Script/Engine.KismetMaterialLibrary))
  (Variables|Default|SetMID_Yields _returnvalue)
  (Rendering|Material|SetMaterial (Variables|Default|GetStaticMesh1) 0 (Variables|Default|GetMID_Yields))
  (CallFunction|UpdateYields (Variables|Default|GetFood) (Variables|Default|GetProd) (Variables|Default|GetGold)))

(fn UpdateYields
  (params (Food :type Integer) (Prod :type Integer) (Gold :type Integer))
  (bind _mid_yields (Variables|Default|GetMID_Yields))
  (bind _mid_yields_2 (Variables|Default|GetMID_Yields))
  (bind _mid_yields_3 (Variables|Default|GetMID_Yields))
  (bind _mid_yields_4 (Variables|Default|GetMID_Yields))
  (bind _mid_yields_5 (Variables|Default|GetMID_Yields))
  (LocalVariables|SetFoodVar Food)
  (LocalVariables|SetProdVar Prod)
  (LocalVariables|SetGoldVar Gold)
  (Rendering|Material|SetScalarParameterValue (Variables|Default|GetMID_Yields) "FoodAmmount" (Math|Conversions|ToFloat(Integer) (LocalVariables|GetFoodVar)) :!class /Script/Engine.MaterialInstanceDynamic)
  (Rendering|Material|SetScalarParameterValue (Variables|Default|GetMID_Yields) "HammerAmmount" (Math|Conversions|ToFloat(Integer) (LocalVariables|GetProdVar)) :!class /Script/Engine.MaterialInstanceDynamic)
  (Rendering|Material|SetScalarParameterValue (Variables|Default|GetMID_Yields) "GoldAmmount" (Math|Conversions|ToFloat(Integer) (LocalVariables|GetGoldVar)) :!class /Script/Engine.MaterialInstanceDynamic)
  (if (and (and (> (LocalVariables|GetFoodVar) 0) (> (LocalVariables|GetProdVar) 0)) (> (LocalVariables|GetGoldVar) 0))
    (Rendering|Material|SetScalarParameterValue _mid_yields_5 "Food_X_Offset" -0.25 :!class /Script/Engine.MaterialInstanceDynamic)
    (Rendering|Material|SetScalarParameterValue _mid_yields_5 "Food_Y_Offset" -0.1 :!class /Script/Engine.MaterialInstanceDynamic)
    (Rendering|Material|SetScalarParameterValue _mid_yields_5 "Hammer_X_Offset" 0.0 :!class /Script/Engine.MaterialInstanceDynamic)
    (Rendering|Material|SetScalarParameterValue _mid_yields_5 "Hammer_Y_Offset" -0.4 :!class /Script/Engine.MaterialInstanceDynamic)
    (Rendering|Material|SetScalarParameterValue _mid_yields_5 "Gold_X_Offset" -0.5 :!class /Script/Engine.MaterialInstanceDynamic)
    (Rendering|Material|SetScalarParameterValue _mid_yields_5 "Gold_Y_Offset" -0.4 :!class /Script/Engine.MaterialInstanceDynamic)
    (elif (and (and (> (LocalVariables|GetFoodVar) 0) (> (LocalVariables|GetProdVar) 0)) (== (LocalVariables|GetGoldVar) 0))
      (Rendering|Material|SetScalarParameterValue _mid_yields_3 "Food_X_Offset" 0.0 :!class /Script/Engine.MaterialInstanceDynamic)
      (Rendering|Material|SetScalarParameterValue _mid_yields_3 "Food_Y_Offset" -0.25 :!class /Script/Engine.MaterialInstanceDynamic)
      (Rendering|Material|SetScalarParameterValue _mid_yields_3 "Hammer_X_Offset" -0.5 :!class /Script/Engine.MaterialInstanceDynamic)
      (Rendering|Material|SetScalarParameterValue _mid_yields_3 "Hammer_Y_Offset" -0.25 :!class /Script/Engine.MaterialInstanceDynamic)
      (elif (and (and (> (LocalVariables|GetFoodVar) 0) (> (LocalVariables|GetGoldVar) 0)) (== (LocalVariables|GetProdVar) 0))
        (Rendering|Material|SetScalarParameterValue _mid_yields_4 "Food_X_Offset" 0.0 :!class /Script/Engine.MaterialInstanceDynamic)
        (Rendering|Material|SetScalarParameterValue _mid_yields_4 "Food_Y_Offset" -0.25 :!class /Script/Engine.MaterialInstanceDynamic)
        (Rendering|Material|SetScalarParameterValue _mid_yields_4 "Gold_X_Offset" -0.5 :!class /Script/Engine.MaterialInstanceDynamic)
        (Rendering|Material|SetScalarParameterValue _mid_yields_4 "Gold_Y_Offset" -0.25 :!class /Script/Engine.MaterialInstanceDynamic)
        (elif (and (and (> (LocalVariables|GetProdVar) 0) (> (LocalVariables|GetGoldVar) 0)) (== (LocalVariables|GetFoodVar) 0))
          (Rendering|Material|SetScalarParameterValue _mid_yields "Hammer_X_Offset" 0.0 :!class /Script/Engine.MaterialInstanceDynamic)
          (Rendering|Material|SetScalarParameterValue _mid_yields "Hammer_Y_Offset" -0.25 :!class /Script/Engine.MaterialInstanceDynamic)
          (Rendering|Material|SetScalarParameterValue _mid_yields "Gold_X_Offset" -0.5 :!class /Script/Engine.MaterialInstanceDynamic)
          (Rendering|Material|SetScalarParameterValue _mid_yields "Gold_Y_Offset" -0.25 :!class /Script/Engine.MaterialInstanceDynamic)
          (else
            (Rendering|Material|SetScalarParameterValue _mid_yields_2 "Food_X_Offset" -0.25 :!class /Script/Engine.MaterialInstanceDynamic)
            (Rendering|Material|SetScalarParameterValue _mid_yields_2 "Food_Y_Offset" -0.25 :!class /Script/Engine.MaterialInstanceDynamic)
            (Rendering|Material|SetScalarParameterValue _mid_yields_2 "Hammer_X_Offset" -0.25 :!class /Script/Engine.MaterialInstanceDynamic)
            (Rendering|Material|SetScalarParameterValue _mid_yields_2 "Hammer_Y_Offset" -0.25 :!class /Script/Engine.MaterialInstanceDynamic)
            (Rendering|Material|SetScalarParameterValue _mid_yields_2 "Gold_X_Offset" -0.25 :!class /Script/Engine.MaterialInstanceDynamic)
            (Rendering|Material|SetScalarParameterValue _mid_yields_2 "Gold_Y_Offset" -0.25 :!class /Script/Engine.MaterialInstanceDynamic)))))))